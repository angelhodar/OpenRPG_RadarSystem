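; BP_DemoMonster is a demo monster character that wanders around its spawn point and describes itself as a movable, non-scannable Monster marker through GetMarkerData.
; On BeginPlay it starts a patrol loop: AIMoveTo a random reachable navmesh point within PatrolRadius, wait, then repeat, with no retry on failure.
; The construction script sizes PatrolSphere to that radius and applies MovementSpeed as walk speed.
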(event `self.ReceiveBeginPlay`
  ;[0.05157 0.3873 1] Just simple AI moving stuff (needs NavMeshBoundVolume in the level)
  (set `self.StartLocation` (`self.K2_GetActorLocation`))
  (`self.StartPatrolling`))

(event `StartPatrolling`
  ;[0.05157 0.3873 1] Just simple AI moving stuff (needs NavMeshBoundVolume in the level)
  (`|AIMoveTo` self (`NavigationSystemV1.K2_GetRandomReachablePointInRadius` (`self.StartLocation`) (`self.PatrolRadius`) null null) null
    (:`OnSuccess`
      (`KismetSystemLibrary.Delay` (`self.PatrolDelay`))
      (`self.StartPatrolling`))))

(fn `GetMarkerData`
  (returns (ID :type Name) (MarkerType :type Name) (`Movable?` :type Boolean) (`CanBeScanned?` :type Boolean))
  (return "None" "Monster" true false))

(fn `UserConstructionScript`
  (`SphereComponent.SetSphereRadius` (`self.PatrolSphere`) (`self.PatrolRadius`) true)
  (set `CharacterMovementComponent.MaxWalkSpeed` (`self.MovementSpeed`) (`self.CharacterMovement`)))