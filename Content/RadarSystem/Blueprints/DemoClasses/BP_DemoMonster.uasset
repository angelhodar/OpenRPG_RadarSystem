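; Demo monster for the radar system that patrols random reachable points around its spawn location.
; On successful AIMoveTo it waits a delay, then picks the next point.
; Its radar sphere adds or removes a marker on the overlapping actor's BPC_RadarHandler, and Tick refreshes that radar's marker distances and positions while in range.
; The construction script applies patrol radius, radar radius and walk speed from variables.
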(event `self.ReceiveBeginPlay`
  (set `self.StartLocation` (`self.K2_GetActorLocation`))
  (`self.StartPatrolling`))

(event `StartPatrolling`
  (`|AIMoveTo` self (`NavigationSystem.K2_GetRandomReachablePointInRadius` (`self.StartLocation`) (`self.PatrolRadius`))
    (:`OnSuccess`
      (`KismetSystemLibrary.Delay` (`self.PatrolDelay`))
      (`self.StartPatrolling`))))

(event `self.RadarColision.OnComponentBeginOverlap`
  (params (OverlappedComponent :type "PrimitiveComponent Object Reference") (OtherActor :type "Actor Object Reference") (OtherComp :type "PrimitiveComponent Object Reference") (OtherBodyIndex :type Integer) (bFromSweep :type Boolean) (SweepResult :type "HitResult Structure (by ref)"))
  (bind _returnvalue (`self.GetComponentByClass` OtherActor "/Game/RadarSystem/Blueprints/BPC_RadarHandler.BPC_RadarHandler_C"))
  (`/Engine/EditorBlueprintResources/StandardMacros.IsValid` _returnvalue
    (:`Is Valid`
      (bind _output_get (set `self.PlayerRadar` _returnvalue))
      (`/Game/RadarSystem/Blueprints/BPC_RadarHandler.AddNewMarker` _output_get (make `/Game/RadarSystem/Structs/s_MarkerInfo` "NewEnumerator2" (0.0 0.0 0.0) self true true false (make `Margin` 0.0 0.0 0.0 6.0))))))

(event `self.RadarColision.OnComponentEndOverlap`
  (params (OverlappedComponent :type "PrimitiveComponent Object Reference") (OtherActor :type "Actor Object Reference") (OtherComp :type "PrimitiveComponent Object Reference") (OtherBodyIndex :type Integer))
  (bind _returnvalue (`self.GetComponentByClass` OtherActor "/Game/RadarSystem/Blueprints/BPC_RadarHandler.BPC_RadarHandler_C"))
  (`/Engine/EditorBlueprintResources/StandardMacros.IsValid` _returnvalue
    (:`Is Valid`
      (`/Game/RadarSystem/Blueprints/BPC_RadarHandler.RemoveMarkerByAttachedActor` _returnvalue self)
      (set `self.PlayerRadar` null))))

(event `self.ReceiveTick`
  (params (DeltaSeconds :type "Float (single-precision)"))
  (bind _playerradar (`self.PlayerRadar`))
  (`/Engine/EditorBlueprintResources/StandardMacros.IsValid` _playerradar
    (:`Is Valid`
      (`/Game/RadarSystem/Blueprints/BPC_RadarHandler.UpdateMarkerDistances` _playerradar)
      (`/Game/RadarSystem/Blueprints/BPC_RadarHandler.UpdateMarkerPositions` _playerradar))))

(fn `UserConstructionScript`
  (`SphereComponent.SetSphereRadius` (`self.PatrolSphere`) (`self.PatrolRadius`) true)
  (set `CharacterMovementComponent.MaxWalkSpeed` (`self.MovementSpeed`) (`self.CharacterMovement`))
  (`SphereComponent.SetSphereRadius` (`self.RadarColision`) (`self.RadarRadius`) true))