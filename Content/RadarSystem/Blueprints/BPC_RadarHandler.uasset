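; Component that drives a horizontal compass-style radar widget showing directions and markers relative to the player's camera.
; Player turn and move events refresh widget positions, marker distances and elevation arrows while visible.
; Yaw deltas, scaled by camera FOV, become horizontal translations; out-of-sight markers either hide or clamp to the edges.
; It also adds and removes markers, toggles visibility with an optional fade, and highlights the radar while registered actors are nearby.
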(event `Initialize`
  (params (Player :type "Actor Object Reference") (Camera :type "CameraComponent Object Reference") (RadarWidget :type "/Game/RadarSystem/UI/WB_Radar Object Reference"))
  ;[0.1284 0.6408 1] Initializes the radar, it needs the player, its camera and the radar widget as inputs
  (set `self.Player` Player)
  (set `self.PlayerCamera` Camera)
  (set `self.RadarWidget` RadarWidget)
  (`self.SetupDefaultDirectionsAndMarkers`)
  (`self.UpdateRadar`))

(event `SetVisibility`
  (params (`Animated?` :type Boolean))
  ;[0.1303 1 0.1921] Handles the radar visibility with its animation
  (if `Animated?`
    (if (`self.Visible?`)
      (`self.UpdateRadar`)
      (`Widget.SetVisibility` (`self.RadarWidget`) "SelfHitTestInvisible")
      (`self.PlayWidgetFadeAnimation` "Reverse"
        (:`Out`
          (set `self.CanChangeVisibility?` true)))
      (else
        (`self.PlayWidgetFadeAnimation` "Forward"
          (:`Out`
            (`Widget.SetVisibility` (`self.RadarWidget`) "Hidden")
            (set `self.CanChangeVisibility?` true)))))
    (else
      (if (`self.Visible?`)
        (`self.UpdateRadar`))
      (`Widget.SetVisibility` (`self.RadarWidget`) (select `bool` (`self.Visible?`) :`false` "Hidden" :`true` "SelfHitTestInvisible" :!type "ESlateVisibility Enum"))
      (set `self.CanChangeVisibility?` true))))

(event `OnPlayerTurned`
  ;[1 0.1927 0.1927] Both events are called from the player every frame (when needed) and updates the radar direction widgets, the markers, etc...
  (if (`self.Visible?`)
    (`self.UpdateDirectionPositions`)
    (`self.UpdateMarkerPositions`)))

(event `OnPlayerMoved`
  ;[1 0.1927 0.1927] Both events are called from the player every frame (when needed) and updates the radar direction widgets, the markers, etc...
  (if (`self.Visible?`)
    (`self.UpdateMarkerDistances`)
    (`self.UpdateMarkerPositions`)
    (`self.UpdateMarkerElevationArrows`)))

(fn `AddHighLightActor`
  (params (Actor :type "Actor Object Reference"))
  (locals (LocalActor :type "Actor Object Reference"))
  (bind _output_get (set `local.LocalActor` Actor))
  (if (`KismetArrayLibrary.Array_Contains` (`self.NearbyHighLightActors`) _output_get)
    (return)
    (else
      (bind _returnvalue (`KismetArrayLibrary.Array_Add` (`self.NearbyHighLightActors`) (`local.LocalActor`)))
      (if (== _returnvalue 0)
        (`/Game/RadarSystem/UI/WB_Radar.ToggleHighLight` (`self.RadarWidget`) true)
        (return)
        (else
          (return))))))

(fn `AddNewDirection`
  (params (Direction :type "/Game/RadarSystem/Structs/s_Direction Structure"))
  (locals (LocalDirection :type "/Game/RadarSystem/Structs/s_Direction Structure"))
  (bind _output_get (set `local.LocalDirection` Direction))
  (`KismetArrayLibrary.Array_Add` (`self.Directions`) _output_get)
  (`/Engine/EditorBlueprintResources/StandardMacros.IsValid` (`self.RadarWidget`)
    (:`Is Valid`
      (`/Game/RadarSystem/UI/WB_Radar.AddDirection` (`self.RadarWidget`) (`local.LocalDirection`))
      (return))
    (:`Is Not Valid`
      (return))))

(fn `AddNewMarker`
  (params (NewMarker :type "/Game/RadarSystem/Structs/s_MarkerInfo Structure"))
  (locals (LocalMarker :type "/Game/RadarSystem/Structs/s_MarkerInfo Structure"))
  (bind _output_get (set `local.LocalMarker` NewMarker))
  (`KismetArrayLibrary.Array_Add` (`self.Markers`) _output_get)
  (`/Engine/EditorBlueprintResources/StandardMacros.IsValid` (`self.RadarWidget`)
    (:`Is Valid`
      (`/Game/RadarSystem/UI/WB_Radar.AddMarker` (`self.RadarWidget`) (`local.LocalMarker`))
      (return))
    (:`Is Not Valid`
      (return))))

(fn `GetDeltaClockWise`
  (params (A :type "Float (double-precision)") (B :type "Float (double-precision)") (`Clockwise?` :type Boolean))
  (returns (Delta :type "Float (double-precision)"))
  (locals (LocalA :type "Float (double-precision)") (LocalB :type "Float (double-precision)"))
  (bind _locala (`local.LocalA`))
  (set `local.LocalA` (mod A 360.0))
  (set `local.LocalB` (mod B 360.0))
  (if `Clockwise?`
    (`/Engine/EditorBlueprintResources/StandardMacros.CompareFloat` (`local.LocalA`) (`local.LocalB`)
      (:`>`
        (return (- 360.0 (- (`local.LocalA`) (`local.LocalB`)))))
      (:`==`
        (return 0.0))
      (:`<`
        (return (- (`local.LocalB`) _locala))))
    (else
      (`/Engine/EditorBlueprintResources/StandardMacros.CompareFloat` (`local.LocalA`) (`local.LocalB`)
        (:`>`
          (return (- _locala (`local.LocalB`))))
        (:`==`
          (return 0.0))
        (:`<`
          (return (- 360.0 (- (`local.LocalB`) (`local.LocalA`)))))))))

(fn `RemoveHighLightActor`
  (params (Actor :type "Actor Object Reference"))
  (locals (LocalActor :type "Actor Object Reference"))
  (bind _output_get (set `local.LocalActor` Actor))
  (if (`KismetArrayLibrary.Array_Contains` (`self.NearbyHighLightActors`) _output_get)
    (`KismetArrayLibrary.Array_RemoveItem` (`self.NearbyHighLightActors`) (`local.LocalActor`))
    (if (== (`KismetArrayLibrary.Array_Length` (`self.NearbyHighLightActors`)) 0)
      (`/Game/RadarSystem/UI/WB_Radar.ToggleHighLight` (`self.RadarWidget`) false)
      (else
        (return)))
    (else
      (return))))

(fn `RemoveMarkerByAttachedActor`
  (params (Actor :type "Actor Object Reference"))
  (locals (LocalActor :type "Actor Object Reference") (LocalRemoveIndex :type Integer :default -1))
  (set `local.LocalActor` Actor)
  (for (_array_element _array_index) (`self.Markers`)
    (if (== (`.AttachedActor_12_181321E84F993F07312BD68E2AE00663` (break `/Game/RadarSystem/Structs/s_MarkerInfo` _array_element)) (`local.LocalActor`))
      (set `local.LocalRemoveIndex` _array_index)))
  (if (!= (`local.LocalRemoveIndex`) -1)
    (`KismetArrayLibrary.Array_Remove` (`self.Markers`) (`local.LocalRemoveIndex`))
    (`Widget.RemoveFromParent` (`|GetArrayItem` (`/Game/RadarSystem/UI/WB_Radar.Markers` (`self.RadarWidget`)) (`local.LocalRemoveIndex`)))
    (`KismetArrayLibrary.Array_Remove` (`/Game/RadarSystem/UI/WB_Radar.Markers` (`self.RadarWidget`)) (`local.LocalRemoveIndex`))
    (return)
    (else
      (return))))

(fn `RemoveMarkerByLocation`
  (params (Location :type "Vector Structure"))
  (locals (LocalActor :type "Actor Object Reference") (LocalRemoveIndex :type Integer :default -1) (LocalLocation :type "Vector Structure"))
  (set `local.LocalLocation` Location)
  (for (_array_element _array_index) (`self.Markers`)
    (if (== (`.StaticLocation_11_2FC8BA1C4B230C4579085587A9AA45A1` (break `/Game/RadarSystem/Structs/s_MarkerInfo` _array_element)) (`local.LocalLocation`))
      (set `local.LocalRemoveIndex` _array_index)))
  (if (!= (`local.LocalRemoveIndex`) -1)
    (`KismetArrayLibrary.Array_Remove` (`self.Markers`) (`local.LocalRemoveIndex`))
    (`Widget.RemoveFromParent` (`|GetArrayItem` (`/Game/RadarSystem/UI/WB_Radar.Markers` (`self.RadarWidget`)) (`local.LocalRemoveIndex`)))
    (`KismetArrayLibrary.Array_Remove` (`/Game/RadarSystem/UI/WB_Radar.Markers` (`self.RadarWidget`)) (`local.LocalRemoveIndex`))
    (return)
    (else
      (return))))

(fn `RotationToCircleDegrees`
  (params (Rotation :type "Float (double-precision)"))
  (returns (CircleDegrees :type "Float (double-precision)"))
  (locals (LocalRotation :type "Float (double-precision)"))
  (bind _output_get (set `local.LocalRotation` Rotation))
  (return (`KismetMathLibrary.SelectFloat` _output_get (mod (+ (`local.LocalRotation`) 360.0) 360.0) (>= (`local.LocalRotation`) 0.0))))

(fn `RotationToTranslation`
  (params (`Rotation A` :type "Rotator Structure") (`Rotation B` :type "Rotator Structure"))
  (returns (Translation :type "Vector2D Structure") (`Clockwise?` :type Boolean) (`OnRadarSight?` :type Boolean))
  (locals (LocalClockwiseDelta :type "Float (double-precision)" :default 0.0) (LocalAntiClockwiseDelta :type "Float (double-precision)" :default 0.0))
  (bind _circledegrees (`self.RotationToCircleDegrees` (.yaw `Rotation B`)))
  (bind _circledegrees_2 (`self.RotationToCircleDegrees` (.yaw `Rotation A`)))
  (bind _returnvalue (/ (`local.LocalAntiClockwiseDelta`) (`CameraComponent.FieldOfView` (`self.PlayerCamera`))))
  (bind _returnvalue_2 (/ (`local.LocalClockwiseDelta`) (`CameraComponent.FieldOfView` (`self.PlayerCamera`))))
  (set `local.LocalClockwiseDelta` (`self.GetDeltaClockWise` _circledegrees_2 _circledegrees true))
  (set `local.LocalAntiClockwiseDelta` (`self.GetDeltaClockWise` _circledegrees_2 _circledegrees))
  (`/Engine/EditorBlueprintResources/StandardMacros.CompareFloat` (`local.LocalClockwiseDelta`) (`local.LocalAntiClockwiseDelta`)
    (:`>`
      (if (<= _returnvalue 1.0)
        (return (`KismetMathLibrary.MakeVector2D` (* (`KismetMathLibrary.Lerp` 0.0 (`self.MaxWidgetTranslation`) _returnvalue) -1.0)) false true)
        (else
          (return (0.0 0.0) false false))))
    (:`==`
      _)
    (:`<`
      _))
  (if (<= _returnvalue_2 1.0)
    (return (`KismetMathLibrary.MakeVector2D` (`KismetMathLibrary.Lerp` 0.0 (`self.MaxWidgetTranslation`) _returnvalue_2)) true true)
    (else
      (return (0.0 0.0) true false))))

(fn `SetupDefaultDirectionsAndMarkers`
  (for _array_element (`self.Directions`)
    (`/Game/RadarSystem/UI/WB_Radar.AddDirection` (`self.RadarWidget`) _array_element))
  (for _array_element_2 (`self.Markers`)
    (`/Game/RadarSystem/UI/WB_Radar.AddMarker` (`self.RadarWidget`) _array_element_2))
  (return))

(fn `ToggleVisibility`
  (params (`Animated?` :type Boolean))
  (if (`self.CanChangeVisibility?`)
    (set `self.CanChangeVisibility?` false)
    (set `self.Visible?` (not (`self.Visible?`)))
    (`self.SetVisibility` `Animated?`)
    (return)))

(fn `UpdateDirectionPositions`
  (locals (LocalDirectionWidget :type "/Game/RadarSystem/UI/WB_Direction Object Reference") (LocalTraslation :type "Vector2D Structure") (LocalOnRadarSight :type Boolean :default false) (LocalWorldRotation :type Integer))
  (bind _localdirectionwidget (`local.LocalDirectionWidget`))
  (bind _returnvalue (`Widget.IsVisible` (`local.LocalDirectionWidget`)))
  (bind (_translation _clockwise_ _onradarsight_) (`self.RotationToTranslation` (`SceneComponent.K2_GetComponentRotation` (`self.PlayerCamera`)) (`KismetMathLibrary.MakeRotator` 0.0 0.0 (`KismetMathLibrary.Conv_IntToDouble` (`local.LocalWorldRotation`)))))
  (for (_array_element _array_index) (`/Game/RadarSystem/UI/WB_Radar.Directions` (`self.RadarWidget`))
    (set `local.LocalDirectionWidget` _array_element)
    (set `local.LocalWorldRotation` (`.WorldRotation_5_3ACB813D492CE3061D1EE2A6A0D98929` (break `/Game/RadarSystem/Structs/s_Direction` (`|GetArrayItem` (`self.Directions`) _array_index))))
    (set `local.LocalTraslation` _translation)
    (bind _output_get (set `local.LocalOnRadarSight` _onradarsight_))
    (if _output_get
      (`Widget.SetRenderTranslation` (`local.LocalDirectionWidget`) (`local.LocalTraslation`))
      (if (not _returnvalue)
        (`Widget.SetVisibility` _localdirectionwidget "SelfHitTestInvisible"))
      (elif _returnvalue
        (`Widget.SetVisibility` _localdirectionwidget "Hidden"))))
  (return))

(fn `UpdateMarkerDistances`
  (locals (LocalMarkerWorldLocation :type "Vector Structure") (LocalWidget :type "/Game/RadarSystem/UI/WB_Marker Object Reference") (LocalMarker :type "/Game/RadarSystem/Structs/s_MarkerInfo Structure"))
  (bind ((`AttachedActor_12_181321E84F993F07312BD68E2AE00663` _attachedactor)) (break `/Game/RadarSystem/Structs/s_MarkerInfo` (`local.LocalMarker`)))
  (for (_array_element _array_index) (`/Game/RadarSystem/UI/WB_Radar.Markers` (`self.RadarWidget`))
    (set `local.LocalWidget` _array_element)
    (bind _output_get (set `local.LocalMarker` (`|GetArrayItem` (`self.Markers`) _array_index)))
    (if (`.ShowDistanceFromPlayer?_8_A87F4C95411AEA2AB395BDA758FD5075` (break `/Game/RadarSystem/Structs/s_MarkerInfo` _output_get))
      (`/Engine/EditorBlueprintResources/StandardMacros.IsValid` _attachedactor
        (:`Is Valid`
          (set `local.LocalMarkerWorldLocation` (`Actor.K2_GetActorLocation` _attachedactor)))
        (:`Is Not Valid`
          (set `local.LocalMarkerWorldLocation` (`.StaticLocation_11_2FC8BA1C4B230C4579085587A9AA45A1` (break `/Game/RadarSystem/Structs/s_MarkerInfo` (`local.LocalMarker`))))))
      (`/Game/RadarSystem/UI/WB_Marker.UpdateDistance` (`local.LocalWidget`) (`KismetMathLibrary.Round` (/ (`KismetMathLibrary.VSize` (- (`KismetMathLibrary.MakeVector` (.x (`local.LocalMarkerWorldLocation`)) (.y (`local.LocalMarkerWorldLocation`))) (`KismetMathLibrary.MakeVector` (.x (`Actor.K2_GetActorLocation` (`self.Player`))) (.y (`Actor.K2_GetActorLocation` (`self.Player`)))))) (`self.MetersConversionValue`))) (`self.MaxDisplayDistance`))))
  (return))

(fn `UpdateMarkerElevationArrows`
  (locals (LocalMarkerWorldLocation :type "Vector Structure") (LocalWidget :type "/Game/RadarSystem/UI/WB_Marker Object Reference") (LocalMarker :type "/Game/RadarSystem/Structs/s_MarkerInfo Structure"))
  (bind _elevationrange (`self.ElevationRange`))
  (bind _localwidget (`local.LocalWidget`))
  (bind ((`AttachedActor_12_181321E84F993F07312BD68E2AE00663` _attachedactor)) (break `/Game/RadarSystem/Structs/s_MarkerInfo` (`local.LocalMarker`)))
  (bind _z (.z (`local.LocalMarkerWorldLocation`)))
  (bind _arrowbox (`/Game/RadarSystem/UI/WB_Marker.ArrowBox` (`local.LocalWidget`)))
  (bind _z_2 (.z (`Actor.K2_GetActorLocation` (`self.Player`))))
  (for (_array_element _array_index) (`/Game/RadarSystem/UI/WB_Radar.Markers` (`self.RadarWidget`))
    (set `local.LocalWidget` _array_element)
    (bind _output_get (set `local.LocalMarker` (`|GetArrayItem` (`self.Markers`) _array_index)))
    (if (`.ShowElevationArrow?_21_73364A6A4660514103329C957F2962A4` (break `/Game/RadarSystem/Structs/s_MarkerInfo` _output_get))
      (`/Engine/EditorBlueprintResources/StandardMacros.IsValid` _attachedactor
        (:`Is Valid`
          (set `local.LocalMarkerWorldLocation` (`Actor.K2_GetActorLocation` _attachedactor)))
        (:`Is Not Valid`
          (set `local.LocalMarkerWorldLocation` (`.StaticLocation_11_2FC8BA1C4B230C4579085587A9AA45A1` (break `/Game/RadarSystem/Structs/s_MarkerInfo` (`local.LocalMarker`))))))
      (if (> _z (+ _z_2 _elevationrange))
        (`/Game/RadarSystem/UI/WB_Marker.UpdateArrowDirection` _localwidget true)
        (`Widget.SetVisibility` _arrowbox "SelfHitTestInvisible")
        (elif (< _z (- _z_2 _elevationrange))
          (`/Game/RadarSystem/UI/WB_Marker.UpdateArrowDirection` _localwidget false)
          (`Widget.SetVisibility` _arrowbox "SelfHitTestInvisible")
          (else
            (`Widget.SetVisibility` (`/Game/RadarSystem/UI/WB_Marker.ArrowBox` (`local.LocalWidget`)) "Hidden"))))))
  (return))

(fn `UpdateMarkerPositions`
  (locals (LocalMarkerWidget :type "/Game/RadarSystem/UI/WB_Marker Object Reference") (LocalMarkerWorldLocation :type "Vector Structure") (LocalMarker :type "/Game/RadarSystem/Structs/s_MarkerInfo Structure") (LocalTranslation :type "Vector2D Structure") (LocalClockWise :type Boolean :default false) (LocalOnRadarSight :type Boolean :default false))
  (bind _localmarkerwidget (`local.LocalMarkerWidget`))
  (bind _maxwidgettranslation (`self.MaxWidgetTranslation`))
  (bind ((`StaticLocation_11_2FC8BA1C4B230C4579085587A9AA45A1` _staticlocation) (`AttachedActor_12_181321E84F993F07312BD68E2AE00663` _attachedactor)) (break `/Game/RadarSystem/Structs/s_MarkerInfo` (`local.LocalMarker`)))
  (bind (_translation _clockwise_ _onradarsight_) (`self.RotationToTranslation` (`SceneComponent.K2_GetComponentRotation` (`self.PlayerCamera`)) (`KismetMathLibrary.FindLookAtRotation` (`Actor.K2_GetActorLocation` (`self.Player`)) (`local.LocalMarkerWorldLocation`))))
  (for (_array_element _array_index) (`/Game/RadarSystem/UI/WB_Radar.Markers` (`self.RadarWidget`))
    (set `local.LocalMarkerWidget` _array_element)
    (set `local.LocalMarker` (`|GetArrayItem` (`self.Markers`) _array_index))
    (`/Engine/EditorBlueprintResources/StandardMacros.IsValid` _attachedactor
      (:`Is Valid`
        (set `local.LocalMarkerWorldLocation` (`Actor.K2_GetActorLocation` _attachedactor)))
      (:`Is Not Valid`
        (set `local.LocalMarkerWorldLocation` _staticlocation)))
    (set `local.LocalTranslation` _translation)
    (set `local.LocalClockWise` _clockwise_)
    (set `local.LocalOnRadarSight` _onradarsight_)
    (if (`.HideWhenOutOfSight?_19_BF03082D4F243FD0A887BC9B439B867A` (break `/Game/RadarSystem/Structs/s_MarkerInfo` (`local.LocalMarker`)))
      (if (`local.LocalOnRadarSight`)
        (`Widget.SetRenderTranslation` _localmarkerwidget (`local.LocalTranslation`))
        (if (not (`Widget.IsVisible` _localmarkerwidget))
          (`Widget.SetVisibility` (`local.LocalMarkerWidget`) "SelfHitTestInvisible"))
        (elif (`Widget.IsVisible` (`local.LocalMarkerWidget`))
          (`Widget.SetVisibility` (`local.LocalMarkerWidget`) "Hidden")))
      (else
        (`Widget.SetRenderTranslation` (`local.LocalMarkerWidget`) (select `bool` (`local.LocalOnRadarSight`) :`false` (`KismetMathLibrary.MakeVector2D` (`KismetMathLibrary.SelectFloat` _maxwidgettranslation (* _maxwidgettranslation -1.0) (`local.LocalClockWise`))) :`true` (`local.LocalTranslation`))))))
  (return))

(fn `UpdateRadar`
  (`self.UpdateDirectionPositions`)
  (`self.UpdateMarkerPositions`)
  (`self.UpdateMarkerDistances`)
  (`self.UpdateMarkerElevationArrows`)
  (return))