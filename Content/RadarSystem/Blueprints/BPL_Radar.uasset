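; BPL_Radar is a Blueprint function library of shared helpers for the radar system.
; It fetches the BPC_Radar component from player character 0 and looks up marker type rows in the DT_MarkerTypes data table by name.
; It also converts Unreal units to meters or kilometers based on a metric enum.
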(fn `ConvertUnrealUnitsToMetric`
  (params (Metric :type Name) (UU :type "Float (double-precision)"))
  (returns (Value :type "Float (double-precision)"))
  (locals (LocalMetric :type Name) (LocalUU :type "Float (double-precision)"))
  (bind _output_get (set `local.LocalMetric` Metric))
  (set `local.LocalUU` UU)
  (switch `name` _output_get
    (:`m`
      (return (/ (`local.LocalUU`) 100.0)))
    (:`km`
      (return (/ (`local.LocalUU`) 100000.0)))))

(fn `GetMarkerTypeData`
  (params (MarkerType :type Name))
  (returns (Data :type "/Game/RadarSystem/Structs/s_MarkerTypeData Structure"))
  (bind _returnvalue (`|GetDataTableRow` "/Game/RadarSystem/Datatables/DT_MarkerTypes.DT_MarkerTypes" MarkerType)
    (:`then`
      (return _returnvalue))
    (:`RowNotFound`
      (return))))

(fn `GetPlayerRadar`
  (returns (PlayerRadar :type "/Game/RadarSystem/Blueprints/BPC_Radar Object Reference"))
  (return (`Actor.GetComponentByClass` (`GameplayStatics.GetPlayerCharacter` (`local.__WorldContext`)) "/Game/RadarSystem/Blueprints/BPC_Radar.BPC_Radar_C")))