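; Player component that drives a compass-style radar widget showing directions, actor or location markers, and a nearby-actor highlight.
; It finds the widget by interface and pushes updates through interface messages when the owner reports turning or moving.
; Shortest yaw delta over camera FOV sets each horizontal offset; markers can clamp to the edge and show distance or elevation arrows.
; It also prunes markers of destroyed actors and fades visibility.
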(event `Initialize`
  (params (PlayerCamera :type "CameraComponent Object Reference"))
  ;[0.1284 0.6408 1] Initializes the radar, it needs the player, its camera and the radar widget as inputs
  (set `self.PlayerCamera` PlayerCamera)
  (set `self.Player` (`self.GetOwner`))
  (bind _foundwidgets (`WidgetBlueprintLibrary.GetAllWidgetsWithInterface` "/Game/RadarSystem/Blueprints/Interfaces/BPI_RadarWidgetCommunication.BPI_RadarWidgetCommunication_C"))
  (bind _output_get (set `self.RadarWidget` (`|GetArrayItem` _foundwidgets)))
  (`/Engine/EditorBlueprintResources/StandardMacros.IsValid` _output_get
    (:`Is Valid`
      (`self.SetupDefaultDirectionsAndMarkers`)
      (`self.UpdateRadar`))
    (:`Is Not Valid`
      (`KismetSystemLibrary.PrintString` "The radar UI hasnt been detected, make sure you create the widget that has the radar widget before you call the Initialize event"))))

(event `SetVisibility`
  (params (`Animated?` :type Boolean))
  ;[0.1303 1 0.1921] Handles the radar visibility with its animation
  (if `Animated?`
    (if (`self.Visible?`)
      (`self.UpdateRadar`)
      (`Widget.SetVisibility` (`self.RadarWidget`) "SelfHitTestInvisible")
      (`self.PlayWidgetFadeAnimation` "Reverse"
        (:`Out`
          (set `self.CanChangeVisibility?` true)))
      (else
        (`self.PlayWidgetFadeAnimation` "Forward"
          (:`Out`
            (`Widget.SetVisibility` (`self.RadarWidget`) "Hidden")
            (set `self.CanChangeVisibility?` true)))))
    (else
      (if (`self.Visible?`)
        (`self.UpdateRadar`))
      (`Widget.SetVisibility` (`self.RadarWidget`) (select `bool` (`self.Visible?`) :`false` "Hidden" :`true` "SelfHitTestInvisible" :!type "ESlateVisibility Enum"))
      (set `self.CanChangeVisibility?` true))))

(event `OnPlayerTurned`
  ;[1 0.1927 0.1927] Both events are called from the player every frame (when needed) and updates the radar direction widgets, the markers, etc...
  (if (`self.Visible?`)
    (`self.UpdateDirections`)
    (`self.UpdateMarkerPositions`)
    (`self.CheckDestroyedActors`)))

(event `OnPlayerMoved`
  ;[1 0.1927 0.1927] Both events are called from the player every frame (when needed) and updates the radar direction widgets, the markers, etc...
  (if (`self.Visible?`)
    (`self.UpdateMarkers`)))

(event `UpdatePlayerCamera`
  (params (Camera :type "CameraComponent Object Reference"))
  ;[1 0.5193 0.1054] Updates the player camera with a new one
  (set `self.PlayerCamera` Camera))

(fn `AddHighLightActor`
  (params (Actor :type "Actor Object Reference"))
  (locals (LocalActor :type "Actor Object Reference"))
  (bind _output_get (set `local.LocalActor` Actor))
  (if (`KismetArrayLibrary.Array_Contains` (`self.NearbyHighLightActors`) _output_get)
    (return)
    (else
      (bind _returnvalue (`KismetArrayLibrary.Array_Add` (`self.NearbyHighLightActors`) (`local.LocalActor`)))
      (if (== _returnvalue 0)
        (message `/Game/RadarSystem/Blueprints/Interfaces/BPI_RadarWidgetCommunication.ToggleHighlight` (`self.RadarWidget`) true)
        (return)
        (else
          (return))))))

(fn `AddNewDirection`
  (params (Direction :type "/Game/RadarSystem/Structs/s_Direction Structure"))
  (locals (LocalDirection :type "/Game/RadarSystem/Structs/s_Direction Structure"))
  (bind _output_get (set `local.LocalDirection` Direction))
  (`KismetArrayLibrary.Array_Add` (`self.Directions`) _output_get)
  (message `/Game/RadarSystem/Blueprints/Interfaces/BPI_RadarWidgetCommunication.AddDirectionWidget` (`self.RadarWidget`) (`local.LocalDirection`))
  (return))

(fn `AddNewMarker`
  (params (NewMarker :type "/Game/RadarSystem/Structs/s_MarkerInfo Structure"))
  (locals (LocalMarker :type "/Game/RadarSystem/Structs/s_MarkerInfo Structure"))
  (bind _output_get (set `local.LocalMarker` NewMarker))
  (`KismetArrayLibrary.Array_Add` (`self.Markers`) _output_get)
  (`KismetArrayLibrary.Array_Add` (`self.TrackedActorMarkers`) (`KismetSystemLibrary.IsValid` (`.AttachedActor_12_181321E84F993F07312BD68E2AE00663` (break `/Game/RadarSystem/Structs/s_MarkerInfo` (`local.LocalMarker`)))))
  (message `/Game/RadarSystem/Blueprints/Interfaces/BPI_RadarWidgetCommunication.AddMarkerWidget` (`self.RadarWidget`) (`local.LocalMarker`))
  (return))

(fn `CheckDestroyedActors`
  (locals (LocalCurrentLoopIndex :type Integer))
  (bind (_arrayindex _arrayelement) (`/Engine/EditorBlueprintResources/StandardMacros.ReverseForEachLoop` (`self.Markers`))
    (:`LoopBody`
      (set `local.LocalCurrentLoopIndex` _arrayindex)
      (if (and (not (`KismetSystemLibrary.IsValid` (`.AttachedActor_12_181321E84F993F07312BD68E2AE00663` (break `/Game/RadarSystem/Structs/s_MarkerInfo` _arrayelement)))) (`|GetArrayItem` (`self.TrackedActorMarkers`) (`local.LocalCurrentLoopIndex`)))
        (`self.RemoveMarker` (`local.LocalCurrentLoopIndex`))
        (return)))
    (:`Completed`
      (return))))

(fn `GetDeltaClockWise`
  (params (A :type "Float (double-precision)") (B :type "Float (double-precision)") (`Clockwise?` :type Boolean))
  (returns (Delta :type "Float (double-precision)"))
  (locals (LocalA :type "Float (double-precision)") (LocalB :type "Float (double-precision)"))
  (bind _locala (`local.LocalA`))
  (set `local.LocalA` (mod A 360.0))
  (set `local.LocalB` (mod B 360.0))
  (if `Clockwise?`
    (`/Engine/EditorBlueprintResources/StandardMacros.CompareFloat` (`local.LocalA`) (`local.LocalB`)
      (:`>`
        (return (- 360.0 (- (`local.LocalA`) (`local.LocalB`)))))
      (:`==`
        (return 0.0))
      (:`<`
        (return (- (`local.LocalB`) _locala))))
    (else
      (`/Engine/EditorBlueprintResources/StandardMacros.CompareFloat` (`local.LocalA`) (`local.LocalB`)
        (:`>`
          (return (- _locala (`local.LocalB`))))
        (:`==`
          (return 0.0))
        (:`<`
          (return (- 360.0 (- (`local.LocalB`) (`local.LocalA`)))))))))

(fn `GetMarkerWorldLocation`
  (params (Marker :type "/Game/RadarSystem/Structs/s_MarkerInfo Structure"))
  (returns (WorldLocation :type "Vector Structure"))
  (bind ((`StaticLocation_11_2FC8BA1C4B230C4579085587A9AA45A1` _staticlocation) (`AttachedActor_12_181321E84F993F07312BD68E2AE00663` _attachedactor)) (break `/Game/RadarSystem/Structs/s_MarkerInfo` Marker))
  (`/Engine/EditorBlueprintResources/StandardMacros.IsValid` _attachedactor
    (:`Is Valid`
      (return (`Actor.K2_GetActorLocation` _attachedactor)))
    (:`Is Not Valid`
      (return _staticlocation))))

(fn `RemoveHighLightActor`
  (params (Actor :type "Actor Object Reference"))
  (locals (LocalActor :type "Actor Object Reference"))
  (bind _output_get (set `local.LocalActor` Actor))
  (if (`KismetArrayLibrary.Array_Contains` (`self.NearbyHighLightActors`) _output_get)
    (`KismetArrayLibrary.Array_RemoveItem` (`self.NearbyHighLightActors`) (`local.LocalActor`))
    (if (== (`KismetArrayLibrary.Array_Length` (`self.NearbyHighLightActors`)) 0)
      (message `/Game/RadarSystem/Blueprints/Interfaces/BPI_RadarWidgetCommunication.ToggleHighlight` (`self.RadarWidget`) false)
      (return)
      (else
        (return)))
    (else
      (return))))

(fn `RemoveMarker`
  (params (MarkerIndex :type Integer))
  (`KismetArrayLibrary.Array_Remove` (`self.Markers`) MarkerIndex)
  (`KismetArrayLibrary.Array_Remove` (`self.TrackedActorMarkers`) MarkerIndex)
  (message `/Game/RadarSystem/Blueprints/Interfaces/BPI_RadarWidgetCommunication.RemoveMarkerWidget` (`self.RadarWidget`) MarkerIndex)
  (return))

(fn `RemoveMarkerByAttachedActor`
  (params (Actor :type "Actor Object Reference"))
  (locals (LocalActor :type "Actor Object Reference") (LocalRemoveIndex :type Integer :default -1))
  (set `local.LocalActor` Actor)
  (for (_array_element _array_index) (`self.Markers`)
    (if (== (`.AttachedActor_12_181321E84F993F07312BD68E2AE00663` (break `/Game/RadarSystem/Structs/s_MarkerInfo` _array_element)) (`local.LocalActor`))
      (set `local.LocalRemoveIndex` _array_index) ; -1 by default
      (break)))
  (if (!= (`local.LocalRemoveIndex`) -1)
    (`self.RemoveMarker` (`local.LocalRemoveIndex`))
    (return)
    (else
      (return))))

(fn `RemoveMarkerByLocation`
  (params (Location :type "Vector Structure"))
  (locals (LocalRemoveIndex :type Integer :default -1) (LocalLocation :type "Vector Structure"))
  (set `local.LocalLocation` Location)
  (for (_array_element _array_index) (`self.Markers`)
    (if (== (`.StaticLocation_11_2FC8BA1C4B230C4579085587A9AA45A1` (break `/Game/RadarSystem/Structs/s_MarkerInfo` _array_element)) (`local.LocalLocation`))
      (set `local.LocalRemoveIndex` _array_index) ; -1 by default
      (break)))
  (if (!= (`local.LocalRemoveIndex`) -1)
    (`self.RemoveMarker` (`local.LocalRemoveIndex`))
    (return)
    (else
      (return))))

(fn `RotationToCircleDegrees`
  (params (Rotation :type "Float (double-precision)"))
  (returns (CircleDegrees :type "Float (double-precision)"))
  (locals (LocalRotation :type "Float (double-precision)"))
  (bind _output_get (set `local.LocalRotation` Rotation))
  (return (`KismetMathLibrary.SelectFloat` _output_get (mod (+ (`local.LocalRotation`) 360.0) 360.0) (>= (`local.LocalRotation`) 0.0))))

(fn `RotationToTranslation`
  (params (`Rotation A` :type "Rotator Structure") (`Rotation B` :type "Rotator Structure"))
  (returns (Translation :type "Vector2D Structure") (`Clockwise?` :type Boolean) (`OnRadarSight?` :type Boolean))
  (locals (LocalClockwiseDelta :type "Float (double-precision)" :default 0.0) (LocalAntiClockwiseDelta :type "Float (double-precision)" :default 0.0))
  (bind _circledegrees (`self.RotationToCircleDegrees` (.yaw `Rotation B`)))
  (bind _circledegrees_2 (`self.RotationToCircleDegrees` (.yaw `Rotation A`)))
  (bind _returnvalue (/ (`local.LocalAntiClockwiseDelta`) (`CameraComponent.FieldOfView` (`self.PlayerCamera`))))
  (bind _returnvalue_2 (/ (`local.LocalClockwiseDelta`) (`CameraComponent.FieldOfView` (`self.PlayerCamera`))))
  (set `local.LocalClockwiseDelta` (`self.GetDeltaClockWise` _circledegrees_2 _circledegrees true))
  (set `local.LocalAntiClockwiseDelta` (`self.GetDeltaClockWise` _circledegrees_2 _circledegrees))
  (`/Engine/EditorBlueprintResources/StandardMacros.CompareFloat` (`local.LocalClockwiseDelta`) (`local.LocalAntiClockwiseDelta`)
    (:`>`
      (if (<= _returnvalue 1.0)
        (return (`KismetMathLibrary.MakeVector2D` (* (`KismetMathLibrary.Lerp` 0.0 (`self.MaxWidgetTranslation`) _returnvalue) -1.0)) false true)
        (else
          (return (0.0 0.0) false false))))
    (:`==`
      _)
    (:`<`
      _))
  (if (<= _returnvalue_2 1.0)
    (return (`KismetMathLibrary.MakeVector2D` (`KismetMathLibrary.Lerp` 0.0 (`self.MaxWidgetTranslation`) _returnvalue_2)) true true)
    (else
      (return (0.0 0.0) true false))))

(fn `SetupDefaultDirectionsAndMarkers`
  (for _array_element (`self.Directions`)
    (message `/Game/RadarSystem/Blueprints/Interfaces/BPI_RadarWidgetCommunication.AddDirectionWidget` (`self.RadarWidget`) _array_element))
  (for _array_element_2 (`self.Markers`)
    (message `/Game/RadarSystem/Blueprints/Interfaces/BPI_RadarWidgetCommunication.AddMarkerWidget` (`self.RadarWidget`) _array_element_2))
  (return))

(fn `ToggleVisibility`
  (params (`Animated?` :type Boolean))
  (if (`self.CanChangeVisibility?`)
    (set `self.CanChangeVisibility?` false)
    (set `self.Visible?` (not (`self.Visible?`)))
    (`self.SetVisibility` `Animated?`)
    (return)))

(fn `UpdateDirections`
  (locals (LocalTraslation :type "Vector2D Structure") (LocalOnRadarSight :type Boolean :default false) (LocalWorldRotation :type Integer) (LocalCurrentLoopIndex :type Integer))
  (bind (_translation _clockwise_ _onradarsight_) (`self.RotationToTranslation` (`SceneComponent.K2_GetComponentRotation` (`self.PlayerCamera`)) (`KismetMathLibrary.MakeRotator` 0.0 0.0 (`KismetMathLibrary.Conv_IntToDouble` (`local.LocalWorldRotation`)))))
  (for (_array_element _array_index) (`self.Directions`)
    (set `local.LocalCurrentLoopIndex` _array_index)
    (set `local.LocalWorldRotation` (`.WorldRotation_5_3ACB813D492CE3061D1EE2A6A0D98929` (break `/Game/RadarSystem/Structs/s_Direction` _array_element)))
    (set `local.LocalTraslation` _translation)
    (set `local.LocalOnRadarSight` _onradarsight_)
    (message `/Game/RadarSystem/Blueprints/Interfaces/BPI_RadarWidgetCommunication.UpdateDirectionWidgetPosition` (`self.RadarWidget`) (`local.LocalCurrentLoopIndex`) (`local.LocalTraslation`) (`local.LocalOnRadarSight`)))
  (return))

(fn `UpdateMarkerDistances`
  (locals (LocalMarkerWorldLocation :type "Vector Structure") (LocalMarker :type "/Game/RadarSystem/Structs/s_MarkerInfo Structure") (LocalCurrentLoopIndex :type Integer))
  (for (_array_element _array_index) (`self.Markers`)
    (set `local.LocalMarker` _array_element)
    (set `local.LocalCurrentLoopIndex` _array_index)
    (if (`.ShowDistanceFromPlayer?_8_A87F4C95411AEA2AB395BDA758FD5075` (break `/Game/RadarSystem/Structs/s_MarkerInfo` (`local.LocalMarker`)))
      (bind _output_get (set `local.LocalMarkerWorldLocation` (`self.GetMarkerWorldLocation` (`local.LocalMarker`))))
      (message `/Game/RadarSystem/Blueprints/Interfaces/BPI_RadarWidgetCommunication.UpdateMarkerWidgetDistance` (`self.RadarWidget`) (`local.LocalCurrentLoopIndex`) (`KismetMathLibrary.Round` (/ (`KismetMathLibrary.VSize` (- (`KismetMathLibrary.MakeVector` (.x _output_get) (.y _output_get)) (`KismetMathLibrary.MakeVector` (.x (`Actor.K2_GetActorLocation` (`self.Player`))) (.y (`Actor.K2_GetActorLocation` (`self.Player`)))))) (`self.UnitConversionValue`))) (`self.MaxDisplayDistance`))))
  (return))

(fn `UpdateMarkerElevationArrows`
  (locals (LocalMarkerWorldLocation :type "Vector Structure") (LocalMarker :type "/Game/RadarSystem/Structs/s_MarkerInfo Structure") (LocalCurrentLoopIndex :type Integer) (LocalUp :type Boolean :default false))
  (bind _elevationrange (`self.ElevationRange`))
  (bind _z (.z (`Actor.K2_GetActorLocation` (`self.Player`))))
  (for (_array_element _array_index) (`self.Markers`)
    (bind _output_get (set `local.LocalMarker` _array_element))
    (set `local.LocalCurrentLoopIndex` _array_index)
    (if (`.ShowElevationArrow?_21_73364A6A4660514103329C957F2962A4` (break `/Game/RadarSystem/Structs/s_MarkerInfo` _output_get))
      (bind _output_get_2 (set `local.LocalMarkerWorldLocation` (`self.GetMarkerWorldLocation` (`local.LocalMarker`))))
      (bind _z_2 (.z _output_get_2))
      (bind _returnvalue (> _z_2 (+ _z _elevationrange)))
      (set `local.LocalUp` _returnvalue)
      (if (not (or _returnvalue (< _z_2 (- _z _elevationrange))))
        (message `/Game/RadarSystem/Blueprints/Interfaces/BPI_RadarWidgetCommunication.UpdateMarkerWidgetElevationArrow` (`self.RadarWidget`) (`local.LocalCurrentLoopIndex`) (`local.LocalUp`) true)
        (else
          (message `/Game/RadarSystem/Blueprints/Interfaces/BPI_RadarWidgetCommunication.UpdateMarkerWidgetElevationArrow` (`self.RadarWidget`) (`local.LocalCurrentLoopIndex`) (`local.LocalUp`) false)))))
  (return))

(fn `UpdateMarkerPositions`
  (locals (LocalMarkerWorldLocation :type "Vector Structure") (LocalMarker :type "/Game/RadarSystem/Structs/s_MarkerInfo Structure") (LocalTranslation :type "Vector2D Structure") (LocalClockWise :type Boolean :default false) (LocalOnRadarSight :type Boolean :default false) (LocalCurrentLoopIndex :type Integer))
  (bind _maxwidgettranslation (`self.MaxWidgetTranslation`))
  (bind (_translation _clockwise_ _onradarsight_) (`self.RotationToTranslation` (`SceneComponent.K2_GetComponentRotation` (`self.PlayerCamera`)) (`KismetMathLibrary.FindLookAtRotation` (`Actor.K2_GetActorLocation` (`self.Player`)) (`local.LocalMarkerWorldLocation`))))
  (for (_array_element _array_index) (`self.Markers`)
    (set `local.LocalMarker` _array_element)
    (set `local.LocalCurrentLoopIndex` _array_index)
    (set `local.LocalMarkerWorldLocation` (`self.GetMarkerWorldLocation` (`local.LocalMarker`)))
    (set `local.LocalTranslation` _translation)
    (set `local.LocalClockWise` _clockwise_)
    (set `local.LocalOnRadarSight` _onradarsight_)
    (if (not (`.HideWhenOutOfSight?_19_BF03082D4F243FD0A887BC9B439B867A` (break `/Game/RadarSystem/Structs/s_MarkerInfo` (`local.LocalMarker`))))
      (set `local.LocalTranslation` (select `bool` (`local.LocalOnRadarSight`) :`false` (`KismetMathLibrary.MakeVector2D` (`KismetMathLibrary.SelectFloat` _maxwidgettranslation (* _maxwidgettranslation -1.0) (`local.LocalClockWise`))) :`true` (`local.LocalTranslation`))))
    (message `/Game/RadarSystem/Blueprints/Interfaces/BPI_RadarWidgetCommunication.UpdateMarkerWidgetPosition` (`self.RadarWidget`) (`local.LocalCurrentLoopIndex`) (`local.LocalTranslation`) (`local.LocalOnRadarSight`) (`.HideWhenOutOfSight?_19_BF03082D4F243FD0A887BC9B439B867A` (break `/Game/RadarSystem/Structs/s_MarkerInfo` (`local.LocalMarker`)))))
  (return))

(fn `UpdateMarkers`
  (`self.UpdateMarkerPositions`)
  (`self.UpdateMarkerDistances`)
  (`self.UpdateMarkerElevationArrows`)
  (`self.CheckDestroyedActors`)
  (return))

(fn `UpdateRadar`
  (`self.UpdateDirections`)
  (`self.UpdateMarkerPositions`)
  (`self.UpdateMarkerDistances`)
  (`self.UpdateMarkerElevationArrows`)
  (`self.CheckDestroyedActors`)
  (return))